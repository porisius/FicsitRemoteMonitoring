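; Example Blueprint showing how a third-party mod adds an API endpoint to Ficsit Remote Monitoring (FRM).
; RegisterWithFRM checks that the FRM mod is loaded, then registers "3rdPartyEndpoint" and a callback delegate on its subsystem actor.
; NonFRMEndpoint builds a sample response array from a JSON string and an example struct converted to a JSON object.
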(event EventBeginPlay)

(event EventTick
  (params (DeltaSeconds :type Float%20%28single-precision%29)))

(fn ConstructionScript)

(fn RegisterwithFRM
  (params (__WorldContext :type Object%20Object%20Reference))
  (if (Class|ModLoadingLibrary|IsModLoaded (Subsystems|GetModLoadingLibrary) "FicsitRemoteMonitoring")
    (Class|FicsitRemoteMonitoring|BlueprintEndpoint (Class|SubsystemActorManager|GetSubsystemActor (Subsystems|GetSubsystemActorManager) "/Script/FicsitRemoteMonitoring.FicsitRemoteMonitoring") "3rdPartyEndpoint" false false (EventDispatchers|CreateEvent :!event Non-FRMEndpoint))))

(fn Non-FRMEndpoint
  (params (WorldContext :type Object%20Object%20Reference))
  (bind _returnvalue (Class|BlueprintJsonObject|StructtoJsonObject (Utilities|Struct|MakeExample_Struct "Name" "ClassName" 1.0 418)))
  (return (Utilities|Array|MakeArray (Class|BlueprintJsonValue|FromString "#praiseBen") (Class|BlueprintJsonValue|FromObject _returnvalue))))