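; Blueprint subsystem for the Ficsit Remote Monitoring mod, providing a serial endpoint bridge and game-data helpers.
; When ArduinoKit is loaded, it opens the configured COM port; Tick, throttled by a Delay, passes received text to HandleEndpoint and writes back the reply.
; BIE functions extract drop pod, Lizard Doggo, schematic, power circuit and research node data.
; IconGenerator renders item and building descriptor icons through a render target to PNG files.
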(event EventBeginPlay)

(event EventTick
  (params (DeltaSeconds :type Float%20%28single-precision%29))
  (Utilities|FlowControl|Delay (.serial_delay (stale EventInitSerialDevice _config)))
  (if (Class|ModLoadingLibrary|IsModLoaded (Subsystems|GetModLoadingLibrary) "ArduinoKit")
    (bind _returnvalue (Class|ArduinoKitBP|IsOpen))
    (if _returnvalue
      (bind _returnvalue_2 (Class|ArduinoKitBP|ReadBytes))
      (bind _returnvalue_3 (Class|ArduinoKitBP|StringfromByteArray _returnvalue_2))
      (bind _output_get (Variables|Default|SetSerialBuffer _returnvalue_3))
      (Class|KismetStringLibrary|ReplaceInline _output_get " 
" "" "IgnoreCase")
      (Math|Integer|CompareInt (Utilities|String|Len _output_get)
        (:>
          (bind _out_data (Class|FicsitRemoteMonitoring|HandleEndpoint :InEndpoint _output_get :Interface "Serial"))
          (Class|ArduinoKitBP|WriteText _out_data))))))

(event EventInitSerialDevice
  (bind _config (|GetModConfiguration))
  (bind _output_get (Variables|Default|SetConfig%20COM%20Port (.com_port _config)))
  (bind _output_get_2 (Variables|Default|SetConfig%20Baud%20Rate (.baud_rate _config)))
  (bind _output_get_3 (Variables|Default|SetConfig%20Serial%20Stack%20Size (.serialstacksize _config)))
  (if (Class|ModLoadingLibrary|IsModLoaded (Subsystems|GetModLoadingLibrary) "ArduinoKit")
    (Class|ArduinoKitBP|Open _output_get _output_get_2 _output_get_3)))

(event EventEndPlay
  (params (EndPlayReason :type EEndPlayReason%20Enum :default "Destroyed"))
  (if (Class|ModLoadingLibrary|IsModLoaded (Subsystems|GetModLoadingLibrary) "ArduinoKit")
    (bind _returnvalue (Class|ArduinoKitBP|IsOpen))
    (if _returnvalue
      (Class|ArduinoKitBP|Close))))

(event EventStopSerialDevice
  (if (Class|ModLoadingLibrary|IsModLoaded (Subsystems|GetModLoadingLibrary) "ArduinoKit")
    (bind _returnvalue (Class|ArduinoKitBP|IsOpen))
    (if _returnvalue
      (Class|ArduinoKitBP|Close))))

(fn ConstructionScript)

(fn GetDropPodInfoBIE
  (params (Droppod :type FG%20Drop%20Pod%20Object%20Reference))
  (bind _returnvalue (Class|FGDropPod|GetUnlockCost Droppod))
  (bind (_itemclass _amount) (Utilities|Struct|BreakItemAmount (.itemcost _returnvalue)))
  (return _itemclass _amount (.powerconsumption _returnvalue)))

(fn GetDoggoInfoBIE
  (params (Doggo :type Actor%20Object%20Reference))
  (bind _aschar_space_rabbit (Utilities|Casting|CastToChar_SpaceRabbit Doggo))
  (bind _displayname (Default|GetDisplayName _aschar_space_rabbit))
  (return (Utilities|String|ToString(Text) _displayname) (Class|FGInventoryComponent|GetInventoryStacks (Variables|/Game/FactoryGame/Character/Creature/Wildlife/SpaceRabbit/Char_SpaceRabbit.Char_SpaceRabbit_C|GetmInventory _aschar_space_rabbit) false)))

(fn SchematictoRecipesBIE
  (params (WorldContext :type Object%20Object%20Reference) (schematicClass :type FG%20Schematic%20Class%20Reference))
  (bind _recipes (CallFunction|GetRecipesfromSchematic schematicClass))
  (bind _hasunlocks (CallFunction|DoSchematicHasUnlocks schematicClass))
  (return _recipes (Class|FGSchematicManager|IsSchematicPurchased (Class|FGSchematicManager|Get WorldContext) schematicClass 0) _hasunlocks (CallFunction|IsSchematicLockedinAnyWay WorldContext schematicClass) (CallFunction|IsSchematicLockedbyTutorial WorldContext schematicClass) (CallFunction|IsSchematicDependentLocked WorldContext schematicClass) (CallFunction|IsSchematicPhaseLocked WorldContext schematicClass) (CallFunction|IsSchematicPartOfTutorial schematicClass)))

(fn CircuitIDBIE
  (params (Buildable :type FG%20Buildable%20Factory%20Object%20Reference))
  (bind _returnvalue (Class|FGBuildableFactory|GetPowerInfo Buildable))
  (return (Class|FGCircuit|GetCircuitID (Class|FGPowerInfoComponent|GetPowerCircuit _returnvalue)) (Class|FGPowerInfoComponent|GetActualConsumption _returnvalue)))

(fn IconGeneratorBIE
  (bind _returnvalue (Rendering|Material|CreateDynamicMaterialInstance "/FicsitRemoteMonitoring/IconSystem/MM_RenderMaterial.MM_RenderMaterial" "None" "None" :!class /Script/Engine.KismetMaterialLibrary))
  (bind _returnvalue_2 (Rendering|CreateRenderTarget2D 512 512 "RTF_RGBA8" "(R=0.000000,G=0.000000,B=0.000000,A=1.000000)" false true))
  (bind _foundclasses (Class|BlueprintAssetHelperLibrary|FindNativeClassesbyType "/Script/FactoryGame.FGItemDescriptor"))
  (bind _output_get (LocalVariables|SetDescriptors _foundclasses))
  (bind _foundclasses_2 (Class|BlueprintAssetHelperLibrary|FindNativeClassesbyType "/Script/FactoryGame.FGBuildingDescriptor"))
  (Utilities|Array|AppendArray _foundclasses_2 _output_get)
  (for _array_element _output_get
    (bind _asfgitem_descriptor (Utilities|Casting|CastToFGItemDescriptorClass _array_element))
    (if (!= _asfgitem_descriptor "/Game/FactoryGame/Equipment/Trinkets/Desc_Trinket_Alpaca.Desc_Trinket_Alpaca_C")
      (Rendering|ClearRenderTarget2D _returnvalue_2 "(R=0.000000,G=0.000000,B=0.000000,A=0.000000)")
      (Rendering|Material|SetTextureParameterValue _returnvalue "Texture" (Variables|/Script/FactoryGame.FGItemDescriptor|GetmPersistentBigIcon (Class|BlueprintReflectionLibrary|GetClassDefaultObject _asfgitem_descriptor)))
      (Rendering|DrawMaterialtoRenderTarget _returnvalue_2 _returnvalue)
      (Rendering|ExportRenderTarget _returnvalue_2 (Utilities|String|Append (Class|KismetSystemLibrary|GetProjectDirectory) "Mods/FicsitRemoteMonitoring/Icons/") (Utilities|String|Append (Utilities|GetClassDisplayName _asfgitem_descriptor) ".png"))))
  (Class|KismetRenderingLibrary|ReleaseRenderTarget2D _returnvalue_2))

(fn PowerCircuitBIE
  (params (Buildable :type FG%20Buildable%20Factory%20Object%20Reference))
  (bind _returnvalue (Class|FGBuildableFactory|GetPowerInfo Buildable))
  (return (Class|FGPowerInfoComponent|GetPowerCircuit _returnvalue) (Class|FGPowerInfoComponent|GetActualConsumption _returnvalue)))

(fn ResearchTreeNodeUnlockDataBIE
  (params (ResearchTreeNode :type FG%20Research%20Tree%20Node%20Object%20Reference))
  (bind _asbpd_research_tree_node (Utilities|Casting|CastToBPD_ResearchTreeNode ResearchTreeNode))
  (if (stale _bsuccess)
    (for _array_element (.parents (Variables|/Game/FactoryGame/Schematics/Research/BPD_ResearchTreeNode.BPD_ResearchTreeNode_C|GetmNodeDataStruct _asbpd_research_tree_node))
      (Utilities|Array|Add (LocalVariables|GetParentPoints) (Utilities|Struct|MakeIntPoint (.x _array_element) (.y _array_element))))
    (for _array_element_2 (.unhiddenby (Variables|/Game/FactoryGame/Schematics/Research/BPD_ResearchTreeNode.BPD_ResearchTreeNode_C|GetmNodeDataStruct _asbpd_research_tree_node))
      (Utilities|Array|Add (LocalVariables|GetUnhiddenByPoints) (Utilities|Struct|MakeIntPoint (.x _array_element_2) (.y _array_element_2))))
    (return (LocalVariables|GetParentPoints) (LocalVariables|GetUnhiddenByPoints) (Utilities|Struct|MakeIntPoint (.x (.coordinates (Variables|/Game/FactoryGame/Schematics/Research/BPD_ResearchTreeNode.BPD_ResearchTreeNode_C|GetmNodeDataStruct _asbpd_research_tree_node))) (.y (.coordinates (Variables|/Game/FactoryGame/Schematics/Research/BPD_ResearchTreeNode.BPD_ResearchTreeNode_C|GetmNodeDataStruct _asbpd_research_tree_node)))))
    (else
      (return 0 0 (Utilities|Struct|MakeIntPoint 0 0)))))